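; Player character Blueprint that manages health, a held shield and death by ragdoll.
; Any, radial and point damage hit the shield while the controller holds it up, otherwise health, with brief invulnerability windows.
; A custom Damage event divides normal, tech, elemental and void damage by armor, and health hits can roll status inflictions.
; Tick regenerates the shield after delays; a broken shield recovers more slowly to a fifth of maximum before clearing.
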(event EventBeginPlay
  (Variables|Default|SetCurrent%20Player%20Health (Variables|Default|GetMax%20Player%20Health))
  (Variables|Default|SetCurrent%20Shield%20Health (Variables|Default|GetMax%20Shield%20Health))
  (bind _asbase_player_controller (Utilities|Casting|CastToBasePlayerController (Game|GetPlayerController 0)))
  (Variables|Default|SetControllerReference _asbase_player_controller))

(event Game|Damage|EventAnyDamage
  (params (Damage :type Float%20%28single-precision%29) (DamageType :type Damage%20Type%20Object%20Reference) (InstigatedBy :type Controller%20Object%20Reference) (DamageCauser :type Actor%20Object%20Reference))
  ;[1 1 1] Any damage taken, check shield - if shield damage shield, if not then health
  (if (not (Variables|Default|GetInvulnerable?))
    (if (Variables|/Game/BluePrint/Player/BasePlayerController.BasePlayerController_C|GetIs%20Shield%20Pressed (Variables|Default|GetControllerReference))
      (Utilities|CheckShield
        (:true
          (Utilities|CheckHealth :!label _label
            (:true
              ;[1 1 1] Damage player, then kill if needed. Also set brief invuln to avoid over damage
              (Utilities|DamageHealth Damage
                (:Player%20Lived
                  (Variables|Default|SetInvulnerable? true)
                  (Utilities|FlowControl|Delay (Variables|Default|GetInvulnerable%20Timer))
                  (Variables|Default|SetInvulnerable? false))
                (:Player%20Died
                  (CallFunction|PlayerDeath))))
            (:false
              (CallFunction|PlayerDeath))))
        (:false
          ;[1 1 1] Set shield to damage, then timer on regen. Also check if broken then set broken / invuln if needed
          (Variables|Default|SetShield%20Damage%20Taken true)
          (Utilities|DamageShield Damage
            (:true
              (CallFunction|CheckShieldBroken)
              (Variables|Default|SetInvulnerable? true)
              (Utilities|FlowControl|Delay 0.5)
              (Variables|Default|SetInvulnerable? false))
            (:false
              (Utilities|FlowControl|RetriggerableDelay (Variables|Default|GetShield%20Regeneration%20Trigger))
              (Variables|Default|SetShield%20Damage%20Taken false)))))
      (else
        (goto _label)))))

(event Game|Damage|EventRadialDamage
  (params (DamageReceived :type Float%20%28single-precision%29) (DamageType :type Damage%20Type%20Object%20Reference) (Origin :type Vector :default "0, 0, 0") (HitInfo :type Hit%20Result%20Structure%20%28by%20ref%29) (InstigatedBy :type Controller%20Object%20Reference) (DamageCauser :type Actor%20Object%20Reference))
  ;[1 1 1] Any damage taken, check shield - if shield damage shield, if not then health
  (if (not (Variables|Default|GetInvulnerable?))
    (if (Variables|/Game/BluePrint/Player/BasePlayerController.BasePlayerController_C|GetIs%20Shield%20Pressed (Variables|Default|GetControllerReference))
      (Utilities|CheckShield
        (:true
          (Utilities|CheckHealth :!label _label
            (:true
              ;[1 1 1] Damage player, then kill if needed. Also set brief invuln to avoid over damage
              (Utilities|DamageHealth DamageReceived
                (:Player%20Lived
                  (Variables|Default|SetInvulnerable? true)
                  (Utilities|FlowControl|Delay (Variables|Default|GetInvulnerable%20Timer))
                  (Variables|Default|SetInvulnerable? false))
                (:Player%20Died
                  (CallFunction|PlayerDeath))))
            (:false
              (CallFunction|PlayerDeath))))
        (:false
          ;[1 1 1] Set shield to damage, then timer on regen. Also check if broken then set broken / invuln if needed
          (Variables|Default|SetShield%20Damage%20Taken true)
          (Utilities|DamageShield DamageReceived
            (:true
              (CallFunction|CheckShieldBroken)
              (Variables|Default|SetInvulnerable? true)
              (Utilities|FlowControl|Delay 0.5)
              (Variables|Default|SetInvulnerable? false))
            (:false
              (Utilities|FlowControl|RetriggerableDelay (Variables|Default|GetShield%20Regeneration%20Trigger))
              (Variables|Default|SetShield%20Damage%20Taken false)))))
      (else
        (goto _label)))))

(event EventDamage
  (params (Normal%20Damage :type Float%20%28single-precision%29) (Tech%20Damage :type Float%20%28single-precision%29) (Elemental%20Damage :type Float%20%28single-precision%29) (Void%20Damage :type Float%20%28single-precision%29) (Tech%20Infliction%20%25 :type Float%20%28single-precision%29) (Elemental%20Infliction%20%25 :type Float%20%28single-precision%29) (Void%20Infliction%20%25 :type Float%20%28single-precision%29))
  (Variables|Default|SetPre-Armor%20Damage (Utilities|Array|MakeArray Normal%20Damage Tech%20Damage Elemental%20Damage Void%20Damage Tech%20Infliction%20%25 Elemental%20Infliction%20%25 Void%20Infliction%20%25))
  (Utilities|DealDamage))

(event EventTick
  (params (DeltaSeconds :type Float%20%28single-precision%29))
  (bind _shield_regeneration_rate (Variables|Default|GetShield%20Regeneration%20Rate))
  ;[1 1 1] Event Tick to regen shield at proper rate
  (Utilities|FlowControl|Sequence
    (:then_0
      (if (Variables|Default|GetIs%20Shield%20Broken?)
        (Utilities|FlowControl|Delay _shield_regeneration_rate)
        (CallFunction|ShieldRegenBroken)
        (elif (not (Variables|/Game/BluePrint/Player/BasePlayerController.BasePlayerController_C|GetIs%20Shield%20Pressed (Variables|Default|GetControllerReference)))
          (Utilities|FlowControl|Delay _shield_regeneration_rate)
          (CallFunction|ShieldRegen))))))

(event Game|Damage|EventPointDamage
  (params (Damage :type Float%20%28single-precision%29) (DamageType :type Damage%20Type%20Object%20Reference) (HitLocation :type Vector :default "0, 0, 0") (HitNormal :type Vector :default "0, 0, 0") (HitComponent :type Primitive%20Component%20Object%20Reference) (BoneName :type Name :default "None") (ShotFromDirection :type Vector :default "0, 0, 0") (InstigatedBy :type Controller%20Object%20Reference) (DamageCauser :type Actor%20Object%20Reference) (HitInfo :type Hit%20Result%20Structure%20%28by%20ref%29))
  ;[1 1 1] Any damage taken, check shield - if shield damage shield, if not then health
  (if (not (Variables|Default|GetInvulnerable?))
    (if (Variables|/Game/BluePrint/Player/BasePlayerController.BasePlayerController_C|GetIs%20Shield%20Pressed (Variables|Default|GetControllerReference))
      (Utilities|CheckShield
        (:true
          (Utilities|CheckHealth :!label _label
            (:true
              ;[1 1 1] Damage player, then kill if needed. Also set brief invuln to avoid over damage
              (Utilities|DamageHealth Damage
                (:Player%20Lived
                  (Variables|Default|SetInvulnerable? true)
                  (Utilities|FlowControl|Delay (Variables|Default|GetInvulnerable%20Timer))
                  (Variables|Default|SetInvulnerable? false))
                (:Player%20Died
                  (CallFunction|PlayerDeath))))
            (:false
              (CallFunction|PlayerDeath))))
        (:false
          ;[1 1 1] Set shield to damage, then timer on regen. Also check if broken then set broken / invuln if needed
          (Variables|Default|SetShield%20Damage%20Taken true)
          (Utilities|DamageShield Damage
            (:true
              (CallFunction|CheckShieldBroken)
              (Variables|Default|SetInvulnerable? true)
              (Utilities|FlowControl|Delay 0.5)
              (Variables|Default|SetInvulnerable? false))
            (:false
              (Utilities|FlowControl|RetriggerableDelay (Variables|Default|GetShield%20Regeneration%20Trigger))
              (Variables|Default|SetShield%20Damage%20Taken false)))))
      (else
        (goto _label)))))

(fn ConstructionScript
  (|CallParentFunction))

(fn PlayerDeath
  (Pawn|Components|CharacterMovement|DisableMovement (Variables|Character|GetCharacterMovement))
  (Physics|SetSimulatePhysics (Variables|Character|GetMesh) true))

(fn CheckShieldBroken
  (bind _controllerreference (Variables|Default|GetControllerReference))
  (if (<= (Variables|Default|GetCurrent%20Shield%20Health) 0.0)
    (Variables|Default|SetIs%20Shield%20Broken? true)
    (Variables|Default|SetIs%20Shield%20Pressed? false)
    (if (Variables|/Game/BluePrint/Player/BasePlayerController.BasePlayerController_C|GetIsShieldVisible (Variables|Default|GetControllerReference))
      (Rendering|ToggleVisibility (Variables|Default|GetPlayerShield) false)
      (Variables|/Game/BluePrint/Player/BasePlayerController.BasePlayerController_C|SetIsShieldVisible _controllerreference false)
      (Default|ShieldSlowPlayer _controllerreference)
      (Default|ShieldNoCollide _controllerreference))))

(fn ShieldRegen
  (if (not (Variables|Default|GetShield%20Damage%20Taken))
    (if (not (>= (Variables|Default|GetCurrent%20Shield%20Health) (Variables|Default|GetMax%20Shield%20Health)))
      (bind _output_get (Variables|Default|SetCurrent%20Shield%20Health (+ (Variables|Default|GetCurrent%20Shield%20Health) (* (Variables|Default|GetMax%20Shield%20Health) 0.0035))))
      (return _output_get))))

(fn ShieldRegenBroken
  (if (< (Variables|Default|GetCurrent%20Shield%20Health) (* (Variables|Default|GetMax%20Shield%20Health) 0.2))
    (Variables|Default|SetCurrent%20Shield%20Health (+ (Variables|Default|GetCurrent%20Shield%20Health) (* (Variables|Default|GetMax%20Shield%20Health) 0.001)))
    (else
      (Variables|Default|SetIs%20Shield%20Broken? false))))

(fn InflictStatus?
  (params (%25%20Chance%20for%20infliction :type Float%20%28single-precision%29))
  (if (<= %25%20Chance%20for%20infliction 0.0)
    _
    (else
      _))
  (return (Math|Integer|InRange(Integer) (Math|Random|RandomIntegerinRange 1 100) 1 (Math|Float|Truncate %25%20Chance%20for%20infliction))))