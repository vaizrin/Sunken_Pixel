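; Player controller for a top-down character: moves it along world axes and turns it toward the cursor hit each Tick.
; BeginPlay caches the PlayerCharacter and adds the HUD; input toggles the inventory, which locks movement, and opens the pause menu.
; Shield toggles visibility, collision and walk slowdown, and the action key is forwarded to the character.
; Attacks and four-slot weapon cycling only track state and print; dodge and old camera logic are disconnected.
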(event Custom|Free%20Look
  ;[1 1 1] OLD - Input: Freelook
)

(event Custom|DodgeDirection
  (bind _player_character_reference (Variables|Default|GetPlayer%20Character%20Reference))
  (bind _returnvalue (Transformation|GetVelocity _player_character_reference))
  (bind _returnvalue_2 (* _returnvalue 1e+01))
  ;[1 1 1] outdated
  ;;[1 1 1] Dodge Direction
  (if (not (Math|Vector|Equal(Vector) _returnvalue_2 "0, 0, 0" 0.0001))
    (Variables|Default|SetPlayerVector _returnvalue_2)))

(event EventBeginPlay
  ;[0.3929 1 0.3379] Client: Initialize Components
  (Input|DisableInput 0)
  (Utilities|FlowControl|Delay 0.5) ; Since this is not a game state demo, this will fix it for testing
  (CallFunction|InitializePlayer)
  (bind _returnvalue (UserInterface|CreateWidget "/Game/BluePrint/UI/ui_PlayerHUD.ui_PlayerHUD_C"))
  (bind _output_get (Variables|Default|SetReference%20To%20Player%20Hud _returnvalue))
  (UserInterface|Viewport|AddtoViewport _output_get 0)
  (Input|EnableInput 0)
  (Variables|Default|SetbShowMouseCursor true))

(event EventTick
  (params (DeltaSeconds :type Float%20%28single-precision%29))
  (bind _array (Utilities|Array|MakeArray "ObjectTypeQuery9"))
  (bind _hitresult (Class|PlayerController|GetHitResultUnderCursorforObjects _array true))
  ;[1 1 1] Player Mouse Look
  (if (.bblockinghit _hitresult)
    (if (not (Variables|Default|GetIs%20Inventory%20Open))
      (Transformation|SetActorRotation (Pawn|GetControlledPawn) (Math|Rotator|MakeRotator 0.0 0.0 (.yaw (Math|Rotator|FindLookatRotation (Transformation|GetActorLocation (Pawn|GetControlledPawn)) (.location _hitresult))))))))

(event Input|ActionEvents|InputActionInventory
  (params (Key :type Key%20Structure))
  ;[1 1 1] Open / Close Inventory
  (:Pressed
    (if (Variables|Default|GetIs%20Inventory%20Open)
      (Variables|Default|SetIs%20Inventory%20Open false)
      (CallFunction|FreeLook)
      (Variables|Default|SetIs%20Movement%20Locked false)
      (Widget|RemovefromParent (stale _returnvalue))
      (else
        (Variables|Default|SetIs%20Inventory%20Open true)
        (CallFunction|FreeLook)
        (Variables|Default|SetIs%20Movement%20Locked true)
        (bind _returnvalue (UserInterface|CreateWidget "/Game/BluePrint/UI/ui_inventory_hud.ui_inventory_hud_C" self))
        (UserInterface|Viewport|AddtoViewport _returnvalue 0)))))

(event Input|ActionEvents|InputActionAction
  (params (Key :type Key%20Structure))
  ;[1 1 1] Action Key
  (:Pressed
    (Class|IntStatusInterface|ActionKeyPress(Message) (Variables|/Game/BluePrint/Player/PlayerCharacter.PlayerCharacter_C|Getbp_inflictstatus (Variables|Default|GetPlayer%20Character%20Reference)))))

(event Input|ActionEvents|InputActionPause
  (params (Key :type Key%20Structure))
  ;[1 1 1] Input: Pause Game
  (:Pressed
    (Development|PrintString "Pause Pressed")
    (if (not (Variables|Default|GetIsPauseShown))
      (bind _returnvalue (UserInterface|CreateWidget "/Game/BluePrint/UI/ui_PauseMenu.ui_PauseMenu_C"))
      (UserInterface|Viewport|AddtoViewport _returnvalue 0)
      (Input|SetInputModeGameandUI (Game|GetPlayerController 0) _returnvalue "DoNotLock" true)
      (Variables|Default|SetIsPauseShown true)
      (Game|SetGamePaused true))))

(event Input|ActionEvents|InputActionFreeCursorKeyboard
  (params (Key :type Key%20Structure))
  ;[1 1 1] OLD - Input: Freelook
)

(event Input|ActionEvents|InputActionFreeCursorGamepad
  (params (Key :type Key%20Structure))
  ;[1 1 1] OLD - Input: Freelook
)

(event Input|ActionEvents|InputActionDash
  (params (Key :type Key%20Structure))
  ;[1 1 1] outdated
  ;;[1 1 1] Dodge, max of 2x each with their own cooldown. Then add a slight pause when trying to do 2 in a row
)

(event Input|ActionEvents|InputActionShield
  (params (Key :type Key%20Structure))
  (bind _player_character_reference (Variables|Default|GetPlayer%20Character%20Reference))
  (bind _playershield (Variables|/Game/BluePrint/Player/PlayerCharacter.PlayerCharacter_C|GetPlayerShield _player_character_reference))
  ;[1 1 1] Input: Shield
  ;;[1 1 1] Ensure the shield is not broken, then appropriately set the shield status
  (:Pressed
    (if (not (Variables|/Game/BluePrint/Player/PlayerCharacter.PlayerCharacter_C|GetIs%20Shield%20Broken? (Variables|Default|GetPlayer%20Character%20Reference)))
      (Variables|Default|SetIs%20Shield%20Pressed true)
      (if (not (Variables|Default|GetIsShieldVisible))
        ;;[1 1 1] Check if the shield is visible / can collide and adjust as the button is pushed or released
        (Rendering|ToggleVisibility _playershield false)
        (Variables|Default|SetIsShieldVisible true)
        (CallFunction|ShieldSlowPlayer)
        (CallFunction|ShieldNoCollide))))
  (:Released
    (Variables|Default|SetIs%20Shield%20Pressed false)
    (if (Variables|Default|GetIsShieldVisible)
      (Rendering|ToggleVisibility _playershield false)
      (Variables|Default|SetIsShieldVisible false)
      (CallFunction|ShieldSlowPlayer)
      (CallFunction|ShieldNoCollide))))

(event Input|ActionEvents|InputActionAttack1
  (params (Key :type Key%20Structure))
  (bind _is_right_mouse_pressed (Variables|Default|GetIs%20Right%20Mouse%20Pressed))
  (bind _is_shield_pressed (Variables|Default|GetIs%20Shield%20Pressed))
  (bind _is_inventory_open (Variables|Default|GetIs%20Inventory%20Open))
  (bind _returnvalue (or _is_right_mouse_pressed _is_shield_pressed))
  ;[1 1 1] Input: Attacks 1 and 2
  (:Pressed
    (if (not _is_inventory_open)
      (Variables|Default|SetIsLeftMousePressed true)
      (if (not _returnvalue)
        (Development|PrintString "Attack 1 press"))))
  (:Released
    (if (not _is_inventory_open)
      (Variables|Default|SetIsLeftMousePressed false)
      (if (not _returnvalue)
        (Development|PrintString "Attack 1 release")))))

(event Input|ActionEvents|InputActionAttack2
  (params (Key :type Key%20Structure))
  (bind _isleftmousepressed (Variables|Default|GetIsLeftMousePressed))
  (bind _is_inventory_open (Variables|Default|GetIs%20Inventory%20Open))
  (bind _returnvalue (or false _isleftmousepressed))
  ;[1 1 1] Input: Attacks 1 and 2
  (:Pressed
    (if (not _is_inventory_open)
      (Variables|Default|SetIs%20Right%20Mouse%20Pressed true)
      (if (not _returnvalue)
        (Development|PrintString "attack 2 press"))))
  (:Released
    (if (not _is_inventory_open)
      (Variables|Default|SetIs%20Right%20Mouse%20Pressed false)
      (if (not _returnvalue)
        (Development|PrintString "attack 2 release")))))

(event Input|ActionEvents|InputActionWeaponscrollup
  (params (Key :type Key%20Structure))
  ;[1 1 1] Weapon Swap
  (:Pressed
    (switch int (Variables|Default|GetCurrent%20Equipped%20Weapon)
      (:1
        (Variables|Default|SetCurrent%20Equipped%20Weapon 4)
        (Development|PrintString "Weapon 4"))
      (:2
        (Variables|Default|SetCurrent%20Equipped%20Weapon 1)
        (Development|PrintString "Weapon 1"))
      (:3
        (Variables|Default|SetCurrent%20Equipped%20Weapon 2)
        (Development|PrintString "Weapon 2"))
      (:4
        (Variables|Default|SetCurrent%20Equipped%20Weapon 3)
        (Development|PrintString "Weapon 3")))))

(event Input|ActionEvents|InputActionWeaponScrolldown
  (params (Key :type Key%20Structure))
  ;[1 1 1] Weapon Swap
  (:Pressed
    (switch int (Variables|Default|GetCurrent%20Equipped%20Weapon)
      (:1
        (Variables|Default|SetCurrent%20Equipped%20Weapon 2)
        (Development|PrintString "Weapon 2"))
      (:2
        (Variables|Default|SetCurrent%20Equipped%20Weapon 3)
        (Development|PrintString "Weapon 3"))
      (:3
        (Variables|Default|SetCurrent%20Equipped%20Weapon 4)
        (Development|PrintString "Weapon 4"))
      (:4
        (Variables|Default|SetCurrent%20Equipped%20Weapon 1)
        (Development|PrintString "Weapon 1")))))

(event Input|AxisEvents|InputAxisLookUp
  (params (AxisValue :type Float%20%28single-precision%29))
  ;[1 1 1] outdated
  ;;[1 1 1] OLD - Input: Mouse Camera
)

(event Input|AxisEvents|InputAxisTurnRate
  (params (AxisValue :type Float%20%28single-precision%29))
  ;[1 1 1] outdated
  ;;[1 1 1] OLD - Input: Gamepad Camera
)

(event Input|AxisEvents|InputAxisTurn
  (params (AxisValue :type Float%20%28single-precision%29))
  ;[1 1 1] outdated
  ;;[1 1 1] OLD - Input: Mouse Camera
)

(event Input|AxisEvents|InputAxisLookUpRate
  (params (AxisValue :type Float%20%28single-precision%29))
  ;[1 1 1] outdated
  ;;[1 1 1] OLD - Input: Gamepad Camera
)

(event Input|AxisEvents|InputAxisMoveForward
  (params (AxisValue :type Float%20%28single-precision%29))
  (bind _player_character_reference (Variables|Default|GetPlayer%20Character%20Reference))
  ;[0.32 0.6818 1] Input: Character Movement
  (Variables|Default|SetPlayerForwardCheck AxisValue)
  (if (not (Variables|Default|GetIs%20Movement%20Locked))
    (Utilities|IsValid _player_character_reference
      (:Is%20Valid
        (Pawn|Input|AddMovementInput _player_character_reference (* (Math|Vector|GetRightVector "0, 0, 0") -1.0) AxisValue false)))))

(event Input|AxisEvents|InputAxisMoveRight
  (params (AxisValue :type Float%20%28single-precision%29))
  (bind _player_character_reference (Variables|Default|GetPlayer%20Character%20Reference))
  ;[0.32 0.6818 1] Input: Character Movement
  (Variables|Default|SetPlayerRightCheck AxisValue)
  (if (not (Variables|Default|GetIs%20Movement%20Locked))
    (Utilities|IsValid _player_character_reference
      (:Is%20Valid
        (Pawn|Input|AddMovementInput _player_character_reference (Math|Vector|GetForwardVector "0, 0, 0") AxisValue false)))))

(fn ConstructionScript)

(fn InitializePlayer
  ;[1 1 1] Initialize player control, in the future add inventory and hud calls here
  (bind _asplayer_character (Utilities|Casting|CastToPlayerCharacter (Pawn|GetControlledPawn))
    (:then
      (Variables|Default|SetPlayer%20Character%20Reference _asplayer_character)
      (Variables|Default|SetbShowMouseCursor false)
      (Variables|Default|SetIs%20Movement%20Locked false))
    (:CastFailed
      (Development|PrintString "Cast to player failed"))))

(fn StartOfGameMouseHide
  (Input|SetInputModeGameOnly (Game|GetPlayerController 0))
  (Variables|Default|SetbShowMouseCursor false))

(fn ShieldSlowPlayer
  (bind _player_character_reference (Variables|Default|GetPlayer%20Character%20Reference))
  (bind _charactermovement (Variables|/Script/Engine.Character|GetCharacterMovement _player_character_reference))
  (if (Variables|Default|GetIsShieldVisible)
    (Variables|Default|SetCurrent%20Walk%20Speed (Variables|/Script/Engine.CharacterMovementComponent|GetMaxWalkSpeed _charactermovement))
    (Variables|/Script/Engine.CharacterMovementComponent|SetMaxWalkSpeed _charactermovement 1e+02)
    (else
      (Variables|/Script/Engine.CharacterMovementComponent|SetMaxWalkSpeed _charactermovement (Variables|Default|GetCurrent%20Walk%20Speed)))))

(fn ShieldNoCollide
  (bind _player_character_reference (Variables|Default|GetPlayer%20Character%20Reference))
  (bind _playershield (Variables|/Game/BluePrint/Player/PlayerCharacter.PlayerCharacter_C|GetPlayerShield _player_character_reference))
  (if (Variables|Default|GetIsShieldVisible)
    (Collision|SetCollisionEnabled _playershield "QueryAndPhysics")
    (else
      (Collision|SetCollisionEnabled _playershield "NoCollision"))))

(fn DodgeCooldown1
  (Variables|Default|SetDodge2Cooldown true))

(fn DodgeCooldown2
  (Variables|Default|SetDodge1Cooldown true))

(fn ResetDodge1
  (Variables|Default|SetCanDodge1 true))

(fn ResetDodge2
  (Variables|Default|SetCanDodge2 true))

(fn Pickup)

(fn UseItem)