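; Pickup actor for a hydrogen stack that hands its item to the player's inventory on touch.
; A sphere overlap casts to PlayerCharacter and sends ItemInfo to its inventory component through the item transfer interface, then destroys the pickup.
; If the component lacks the interface, it prints an error and the pickup remains.
; The construction script is empty despite its comment about setting the item class automatically.
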(event OnComponentBeginOverlap(Sphere)
  (params (OverlappedComponent :type Primitive%20Component%20Object%20Reference) (OtherActor :type Actor%20Object%20Reference) (OtherComp :type Primitive%20Component%20Object%20Reference) (OtherBodyIndex :type Integer) (bFromSweep :type Boolean) (SweepResult :type Hit%20Result%20Structure%20%28by%20ref%29))
  (Utilities|IsValid OtherActor
    (:Is%20Valid
      (bind _asplayer_character (Utilities|Casting|CastToPlayerCharacter OtherActor))
      (Variables|Default|SetPlayer%20Character%20Ref _asplayer_character)
      (bind _output_get (Variables|Default|SetInventory%20Component%20Ref (Variables|/Game/BluePrint/Player/PlayerCharacter.PlayerCharacter_C|Getbp_player_inventory _asplayer_character)))
      (if (Utilities|DoesObjectImplementInterface _output_get "/Game/BluePrint/Utility/int_item_transfer_interface.int_item_transfer_interface_C")
        (Class|IntItemTransferInterface|ItemTransferEvent(Message) (Variables|Default|GetInventory%20Component%20Ref) (Variables|Default|GetItem%20Info))
        (Actor|DestroyActor)
        (else
          (Development|PrintString "Can Not Transfer Item"))))))

(fn ConstructionScript
  ;[1 1 1] Automatically Set Item Class
)