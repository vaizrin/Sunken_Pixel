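; Inventory component that receives transferred items into an array of item info structs, limited by a total slot count.
; ItemTransferEvent accepts an item only if its stack size plus the current entry count is below the slot limit.
; For stackable items, StackItem searches for an entry with the same name and adds the incoming count to it, without checking the stack limit.
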(event EventItemTransferEvent
  (params (Item%20Info :type S%20Inventory%20Structure))
  (Variables|Default|SetIncoming%20Item%20Info Item%20Info)
  (if (< (+ (.CurrentStack (Utilities|Struct|Breaks_inventory (Variables|Default|GetIncoming%20Item%20Info))) (Utilities|Array|Length (Variables|Default|GetInventory))) (Variables|Default|GetTotal%20Slots))
    (if (.CanStack? (Utilities|Struct|Breaks_inventory (Variables|Default|GetIncoming%20Item%20Info)))
      (Utilities|StackItem (Variables|Default|GetIncoming%20Item%20Info)
        (:false
          _)))
    (Utilities|Array|Add (Variables|Default|GetInventory) (Variables|Default|GetIncoming%20Item%20Info))))