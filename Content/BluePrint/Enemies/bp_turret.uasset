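; Enemy turret that turns toward the player when it senses or takes damage, and is destroyed when its health runs out.
; Both triggers share one path: a timeline lerps rotation toward the last seen player, then after a retriggerable delay another eases it back.
; Sightings, but not hits, fire a delayed three-shell burst on alternate passes via a toggle flag.
; The laser warm-up before firing is disconnected and never runs.
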(event OnSeePawn(PawnSensing)
  (params (Pawn :type Pawn%20Object%20Reference))
  (Variables|Default|SetReacting%20To%20Damage false)
  (bind _asplayer_character (Utilities|Casting|CastToPlayerCharacter Pawn))
  (Utilities|FlowControl|Sequence
    (:then_0
      (bind _0_1_floats (Timeline|Timeline_2 Stop)
        (:Update
          (Transformation|SetActorRotation (Math|Rotator|Lerp(Rotator) (Math|Rotator|FindLookatRotation (Transformation|GetActorLocation) (Transformation|GetActorLocation _asplayer_character)) (Math|Rotator|MakeRotationfromAxes (Variables|Default|GetForward_Vector) (Variables|Default|GetRight_Vector) (Variables|Default|GetUp_Vector)) _0_1_floats true))
          (Components|Activation|Deactivate (Variables|Default|GetLaser%20Spawn%20Point)))))
    (:then_1
      (bind _0_1_floats_2 (Timeline|Timeline_0 PlayFromStart)
        (:Update
          (Transformation|SetActorRotation (Math|Rotator|Lerp(Rotator) (Math|Conversions|RotationFromXVector (Math|Vector|GetForwardVector (Variables|Default|GetTurret%20Mesh))) (Math|Rotator|FindLookatRotation (Transformation|GetActorLocation) (Transformation|GetActorLocation _asplayer_character)) _0_1_floats_2 true))
          (Utilities|FlowControl|RetriggerableDelay 2.0)
          (Timeline|Timeline_2 PlayFromStart))))
    (:then_2
      (if (not (Variables|Default|GetReacting%20To%20Damage))
        (if (Variables|Default|GetSpawn_Projectile)
          (Utilities|FlowControl|Delay (- (Variables|Default|GetFire_Rate) (Variables|Default|GetLaser_On_Time)))
          (Game|SpawnActorfromClass "/Game/BluePrint/Enemies/bp_projectile_shell.bp_projectile_shell_C" (Transformation|GetWorldTransform (Variables|Default|GetProjectile%20Spawn%20Point)) "AdjustIfPossibleButAlwaysSpawn" 0 0)
          (Utilities|FlowControl|Delay 0.2)
          (Game|SpawnActorfromClass "/Game/BluePrint/Enemies/bp_projectile_shell.bp_projectile_shell_C" (Transformation|GetWorldTransform (Variables|Default|GetProjectile%20Spawn%20Point)) "AdjustIfPossibleButAlwaysSpawn" 0 0)
          (Utilities|FlowControl|Delay 0.2)
          (Game|SpawnActorfromClass "/Game/BluePrint/Enemies/bp_projectile_shell.bp_projectile_shell_C" (Transformation|GetWorldTransform (Variables|Default|GetProjectile%20Spawn%20Point)) "AdjustIfPossibleButAlwaysSpawn" 0 0)
          (Variables|Default|SetSpawn_Projectile false)
          (else
            (Variables|Default|SetSpawn_Projectile true)))))))

(event EventDamage
  (params (Normal%20Damage :type Float%20%28single-precision%29) (Tech%20Damage :type Float%20%28single-precision%29) (Elemental%20Damage :type Float%20%28single-precision%29) (Void%20Damage :type Float%20%28single-precision%29) (Tech%20Infliction%20%25 :type Float%20%28single-precision%29) (Elemental%20Infliction%20%25 :type Float%20%28single-precision%29) (Void%20Infliction%20%25 :type Float%20%28single-precision%29))
  ;[1 1 1] Damage Taken
  (Variables|Default|SetReacting%20To%20Damage true)
  (if (> Normal%20Damage (Variables|Default|GetCurrent%20Health))
    (Actor|DestroyActor)
    (else
      (Variables|Default|SetCurrent%20Health (- (Variables|Default|GetCurrent%20Health) 1.0))
      (if (<= (Variables|Default|GetCurrent%20Health) 0.0)
        (Actor|DestroyActor)
        (else
          (Utilities|FlowControl|Sequence
            (:then_0
              (bind _0_1_floats (Timeline|Timeline_2 Stop)
                (:Update
                  (Transformation|SetActorRotation (Math|Rotator|Lerp(Rotator) (Math|Rotator|FindLookatRotation (Transformation|GetActorLocation) (Transformation|GetActorLocation (stale OnSeePawn(PawnSensing) _asplayer_character))) (Math|Rotator|MakeRotationfromAxes (Variables|Default|GetForward_Vector) (Variables|Default|GetRight_Vector) (Variables|Default|GetUp_Vector)) _0_1_floats true))
                  (Components|Activation|Deactivate (Variables|Default|GetLaser%20Spawn%20Point)))))
            (:then_1
              (bind _0_1_floats_2 (Timeline|Timeline_0 PlayFromStart)
                (:Update
                  (Transformation|SetActorRotation (Math|Rotator|Lerp(Rotator) (Math|Conversions|RotationFromXVector (Math|Vector|GetForwardVector (Variables|Default|GetTurret%20Mesh))) (Math|Rotator|FindLookatRotation (Transformation|GetActorLocation) (Transformation|GetActorLocation (stale OnSeePawn(PawnSensing) _asplayer_character))) _0_1_floats_2 true))
                  (Utilities|FlowControl|RetriggerableDelay 2.0)
                  (Timeline|Timeline_2 PlayFromStart))))
            (:then_2
              (if (not (Variables|Default|GetReacting%20To%20Damage))
                (if (Variables|Default|GetSpawn_Projectile)
                  (Utilities|FlowControl|Delay (- (Variables|Default|GetFire_Rate) (Variables|Default|GetLaser_On_Time)))
                  (Game|SpawnActorfromClass "/Game/BluePrint/Enemies/bp_projectile_shell.bp_projectile_shell_C" (Transformation|GetWorldTransform (Variables|Default|GetProjectile%20Spawn%20Point)) "AdjustIfPossibleButAlwaysSpawn" 0 0)
                  (Utilities|FlowControl|Delay 0.2)
                  (Game|SpawnActorfromClass "/Game/BluePrint/Enemies/bp_projectile_shell.bp_projectile_shell_C" (Transformation|GetWorldTransform (Variables|Default|GetProjectile%20Spawn%20Point)) "AdjustIfPossibleButAlwaysSpawn" 0 0)
                  (Utilities|FlowControl|Delay 0.2)
                  (Game|SpawnActorfromClass "/Game/BluePrint/Enemies/bp_projectile_shell.bp_projectile_shell_C" (Transformation|GetWorldTransform (Variables|Default|GetProjectile%20Spawn%20Point)) "AdjustIfPossibleButAlwaysSpawn" 0 0)
                  (Variables|Default|SetSpawn_Projectile false)
                  (else
                    (Variables|Default|SetSpawn_Projectile true)))))))))))

(fn ConstructionScript)