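; Chain-reacting enemy bio bomb that counts down on a text display, then after a three-second delay damages overlapping actors in its blast radius.
; A Camera-channel line trace to each actor must register a hit before DamageMessage sends normal, elemental and infliction damage.
; Each damaged actor may spawn another bomb at its location, with odds shrinking as SpawnChainCount grows.
; The bomb then destroys itself; bombs past the chain limit never arm.
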(event Custom|Start%20Timer
  ;[1 1 1] Find every actor with the status interface and do a visual line trace - if the bomb can see it, hit them
  (Utilities|Time|SetTimerbyFunctionName 0 "Increment Time" (Variables|Default|GetDelta%20Time) true))

(event EventBeginPlay
  ;[1 1 1] Find every actor with the status interface and do a visual line trace - if the bomb can see it, hit them
  (bind _output_get (Variables|Default|SetLocal%20Counter (+ (Variables|Default|GetSpawn%20Chain%20Count) 1)))
  (Development|PrintString (Utilities|String|ToString(Integer) _output_get))
  (if (not (> _output_get 4))
    (CallFunction|StartTimer)
    (Utilities|FlowControl|Delay 3.0)
    (for _array_element (Collision|GetOverlappingActors (Variables|Default|GetBlast%20Radius) "/Game/BluePrint/Player/PlayerCharacter.PlayerCharacter_C" :!class /Script/Engine.PrimitiveComponent)
      (bind _output_get_2 (Variables|Default|SetActor%20Array%20Reference _array_element))
      (if (Collision|IsOverlappingActor (Variables|Default|GetBlast%20Radius) _array_element :!class /Script/Engine.PrimitiveComponent)
        (bind _returnvalue (Collision|LineTraceByChannel (Transformation|GetWorldLocation (Variables|Default|Getbomb%20mesh)) (Transformation|GetActorLocation _output_get_2) "TraceTypeQuery2" false 0 "Persistent" true "(R=1.000000,G=0.000000,B=0.000000,A=1.000000)" "(R=0.000000,G=1.000000,B=0.000000,A=1.000000)" 1e+01))
        (if _returnvalue
          ;[1 1 1] Damage and Spawn BioBomb on Every Actor Hit That Has BP_Status Interface
          (Class|IntDamageInterface|Damage(Message) (Variables|Default|GetActor%20Array%20Reference) (Variables|Default|GetNormal%20Damage) 0.0 (Variables|Default|GetElemental%20Damage) 0.0 0.0 (Variables|Default|GetElemental%20Infliction%20%25) 0.0)
          (if (Math|Integer|InRange(Integer) (Math|Random|RandomIntegerinRange 0 (Variables|Default|GetLocal%20Counter)) 0 1)
            (Game|SpawnActorfromClass "bp_biobomb_C" (Math|Transform|MakeTransform (Transformation|GetActorLocation (Variables|Default|GetActor%20Array%20Reference)) "0, 0, 0" "1,1,1") "Undefined" 0 (Variables|Default|GetLocal%20Counter) 0)))))
    (Actor|DestroyActor)))

(fn ConstructionScript)

(fn IncrementTime
  (bind _output_get (Variables|Default|SetTimer (- (Variables|Default|GetTimer) (Variables|Default|GetDelta%20Time))))
  (if (not (<= _output_get 0.0))
    (Rendering|Components|TextRender|SetText (Variables|Default|GetTimer%20To%20Blow) (Utilities|Text|ToText(Float) (Variables|Default|GetTimer) "HalfToEven" false true 1 324 0 0))))