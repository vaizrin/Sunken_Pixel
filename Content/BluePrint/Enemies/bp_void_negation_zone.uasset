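; Void negation zone actor that tells the player's status-infliction component whether a void-afflicted player is standing inside it.
; A delayed Tick compares player distance to the Sphere's center against a fixed radius, rather than using overlap events, and sends in-zone or out-of-zone messages with the zone's counter.
; An external event supplies player references, and a kill event destroys the zone after a counter-scaled delay, staggering removal by counter value.
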(event EventKillNegationZones
  (params (Status%20Inflict%20Component%20Ref :type Actor%20Component%20Object%20Reference))
  ;[1 1 1] On Event Trigger Kill Self
  (Utilities|FlowControl|Delay (/ (Math|Conversions|ToFloat(Integer) (Variables|Default|GetInt%20Counter)) 2.0))
  (Actor|DestroyActor))

(event EventPlayerandControllerReferenceSet
  (params (Controller%20Reference :type Base%20Player%20Controller%20Object%20Reference) (Player%20Reference :type Player%20Character%20Object%20Reference) (Bp%20Status%20Inflict%20Ref :type Actor%20Component%20Object%20Reference))
  ;[1 1 1] On spawn, set references
  (Variables|Default|SetPlayer%20Controller%20Reference Controller%20Reference)
  (Variables|Default|SetPlayer%20Character%20Reference Player%20Reference)
  (Variables|Default|SetInflict%20Status%20Component%20Reference Bp%20Status%20Inflict%20Ref))

(event EventTick
  (params (DeltaSeconds :type Float%20%28single-precision%29))
  (bind _player_character_reference (Variables|Default|GetPlayer%20Character%20Reference))
  (bind _player_character_reference_2 (Variables|Default|GetPlayer%20Character%20Reference))
  (bind _bp_inflictstatus (Variables|/Game/BluePrint/Player/PlayerCharacter.PlayerCharacter_C|Getbp_inflictstatus _player_character_reference_2))
  ;[1 1 1] Determine if player is close or not
  (Utilities|FlowControl|Delay 0.01)
  (if (or (Variables|/Game/BluePrint/Player/PlayerCharacter.PlayerCharacter_C|GetIs%20Void%20Status%20Inflicted? _player_character_reference) (Variables|/Game/BluePrint/Player/PlayerCharacter.PlayerCharacter_C|GetIs%20Void%20Sick? _player_character_reference))
    (if (>= (Math|Vector|VectorLength (- (Transformation|GetWorldLocation (Variables|Default|GetSphere)) (Transformation|GetActorLocation (Variables|Default|GetPlayer%20Character%20Reference)))) 1.6e+02)
      (Class|IntStatusInterface|VoidZoneEndOverlap(Message) _bp_inflictstatus false (Variables|Default|GetInt%20Counter))
      (Development|PrintString "3")
      (else
        (Class|IntStatusInterface|VoidZoneOverlap(Message) _bp_inflictstatus true (Variables|Default|GetInt%20Counter) self)))))

(fn ConstructionScript)