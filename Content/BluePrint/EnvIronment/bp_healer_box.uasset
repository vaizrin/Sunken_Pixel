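; Health pickup box that heals the player when they overlap it.
; On overlap it casts the other actor to PlayerCharacter and adds HealthAdded to its current health, capped at MaxPlayerHealth, then destroys itself.
; Debug prints report every overlap and any failed cast, and a non-player overlap leaves the box in place.
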(event EventBeginPlay)

(event Collision|EventActorBeginOverlap
  (params (OtherActor :type Actor%20Object%20Reference))
  (Development|PrintString "OVERLAP")
  (bind _asplayer_character (Utilities|Casting|CastToPlayerCharacter OtherActor)
    (:then
      (if (>= (+ (Variables|/Game/BluePrint/Player/PlayerCharacter.PlayerCharacter_C|GetCurrent%20Player%20Health _asplayer_character) (Variables|Default|GetHealthAdded)) (Variables|/Game/BluePrint/Player/PlayerCharacter.PlayerCharacter_C|GetMax%20Player%20Health _asplayer_character))
        (Variables|/Game/BluePrint/Player/PlayerCharacter.PlayerCharacter_C|SetCurrent%20Player%20Health _asplayer_character (Variables|/Game/BluePrint/Player/PlayerCharacter.PlayerCharacter_C|GetMax%20Player%20Health _asplayer_character))
        (else
          (Variables|/Game/BluePrint/Player/PlayerCharacter.PlayerCharacter_C|SetCurrent%20Player%20Health _asplayer_character (+ (Variables|/Game/BluePrint/Player/PlayerCharacter.PlayerCharacter_C|GetCurrent%20Player%20Health _asplayer_character) (Variables|Default|GetHealthAdded)))))
      (Actor|DestroyActor self))
    (:CastFailed
      (Development|PrintString "PLAYER CAST FAILED - HEAL BOX"))))

(event EventTick
  (params (DeltaSeconds :type Float%20%28single-precision%29)))

(fn ConstructionScript)